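; DP_Movement is a player character Blueprint that handles walking, looking and jumping.
; Movement axis inputs feed AddMovementInput along the actor's own forward (X) and right (Y) vectors, rather than the control rotation.
; Camera axis inputs drive controller yaw and pitch, scaled down by a fixed sensitivity factor.
; The jump action calls Jump on press, and the construction script only calls its parent.
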(event `InputAxis|Camera_MovementAxisX`
  (params (AxisValue :type "Float (single-precision)"))
  (`self.AddControllerYawInput` (* AxisValue 0.4)))

(event `InputAxis|MovementAxisX`
  (params (AxisValue :type "Float (single-precision)"))
  (`self.AddMovementInput` (`self.GetActorForwardVector`) AxisValue))

(event `InputAxis|Camera_MovementAxisY`
  (params (AxisValue :type "Float (single-precision)"))
  (`self.AddControllerPitchInput` (* AxisValue 0.4)))

(event `InputAxis|MovementAxisY`
  (params (AxisValue :type "Float (single-precision)"))
  (`self.AddMovementInput` (`self.GetActorRightVector`) AxisValue))

(event `EnhancedInput|/Game/BluePrint/IMC/IA/IA_Jump`
  (params (ActionValue :type Boolean) (ElapsedSeconds :type "Float (double-precision)") (TriggeredSeconds :type "Float (double-precision)") (InputAction :type "InputAction Object Reference" :default "/Game/BluePrint/IMC/IA/IA_Jump.IA_Jump"))
  (:`Triggered`
    (`self.Jump`)))

(fn `UserConstructionScript`
  (`parent.UserConstructionScript`))